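; BP_Enemy is an AI enemy that chases the player and takes points away on reaching them.
; The chase uses AIMoveTo, then a sphere trace at its location calls CEReducePoint on hit third-person characters tagged "player".
; A separate go-away event moves it to a random reachable point, then resumes the chase whether that move succeeds or fails.
; BeginPlay is empty, and neither event is started by it.
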(event `self.ReceiveBeginPlay`)

(event `CE_Chase Player`
  (bind _returnvalue (`self.K2_GetActorLocation`))
  (`|AIMoveTo` self (0.0 0.0 0.0) (`GameplayStatics.GetPlayerCharacter` 0)
    (:`OnSuccess`
      (bind _outhits (`KismetSystemLibrary.SphereTraceMulti` :`Start` _returnvalue :`End` _returnvalue :`TraceChannel` "TraceTypeQuery1" :`DrawDebugType` "ForDuration"))
      (for _array_element _outhits
        (bind (_bblockinghit _binitialoverlap _time _distance _location _impactpoint _normal _impactnormal _physmat _hitactor) (`GameplayStatics.BreakHitResult` _array_element))
        (if (`self.ActorHasTag` _hitactor "player")
          (bind _asbp_third_person_character (cast `/Game/ThirdPerson/Blueprints/BP_ThirdPersonCharacter` _hitactor))
          (`/Game/ThirdPerson/Blueprints/BP_ThirdPersonCharacter.CE_Reduce Point` _asbp_third_person_character))))))

(event `CE_Go Away`
  (`|AIMoveTo` self (`NavigationSystemV1.K2_GetRandomReachablePointInRadius` (`self.K2_GetActorLocation`) 0.0 null null) null
    (:`OnSuccess`
      _)
    (:`OnFail`
      _))
  (`self.CE_Chase Player`))

(fn `UserConstructionScript`)